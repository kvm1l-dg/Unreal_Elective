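; BP_InteractionFire is an interactable fire that needs two logs from the player before it can be lit.
; A collision sphere shows or hides an interaction widget, cached as UI_Interaction on BeginPlay.
; Interact destroys the player's attached log and increments a counter; below two, it sets the widget to the wood text.
; Once fed, interactions alternate through a FlipFlop between activating the fire with cleared text and deactivating it.
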(event OnComponentEndOverlap(Sphere_Collision)
  (params (OverlappedComponent :type Primitive%20Component%20Object%20Reference) (OtherActor :type Actor%20Object%20Reference) (OtherComp :type Primitive%20Component%20Object%20Reference) (OtherBodyIndex :type Integer))
  ;[0.15 0.003125 0.003125 0.5] Widget
  (Rendering|SetVisibility (Variables|Default|GetWidget) false false))

(event OnComponentBeginOverlap(Sphere_Collision)
  (params (OverlappedComponent :type Primitive%20Component%20Object%20Reference) (OtherActor :type Actor%20Object%20Reference) (OtherComp :type Primitive%20Component%20Object%20Reference) (OtherBodyIndex :type Integer) (bFromSweep :type Boolean) (SweepResult :type Hit%20Result%20Structure%20%28by%20ref%29))
  ;[0.15 0.003125 0.003125 0.5] Widget
  (Rendering|SetVisibility (Variables|Default|GetWidget) true false))

(event EventBeginPlay
  ;[0.651 0.3311 0.6096 0.5] Getting the widget and converting the text
  (bind _asui_interaction (Utilities|Casting|CastToUI_Interaction (UserInterface|GetWidget (Variables|Default|GetWidget))))
  (Variables|Default|SetAs%20UI%20Interaction _asui_interaction))

(event Collision|EventActorBeginOverlap
  (params (OtherActor :type Actor%20Object%20Reference)))

(event EventTick
  (params (DeltaSeconds :type Float%20%28single-precision%29)))

(event EventInteract
  (params (PlayerRef :type BP%20First%20Person%20Character%20Object%20Reference))
  ;[1 0.4174 0 0.5] If in hand delete wood
  (if (Variables|/Game/FirstPerson/Blueprints/BP_FirstPersonCharacter.BP_FirstPersonCharacter_C|GetLog%20Attached%20 PlayerRef)
    (Actor|DestroyActor (Variables|/Game/FirstPerson/Blueprints/BP_FirstPersonCharacter.BP_FirstPersonCharacter_C|GetWoodenLog PlayerRef))
    (Variables|/Game/FirstPerson/Blueprints/BP_FirstPersonCharacter.BP_FirstPersonCharacter_C|SetLog%20Attached%20 PlayerRef false)
    (Math|Integer|IncrementInt (Variables|Default|GetLogsPutIn)
      (:%20%20
        _)))
  ;[0.15 0.04278 0.1444 0.5] Activate/Deactivate
  (if (>= (Variables|Default|GetLogsPutIn) 2)
    (Utilities|FlowControl|FlipFlop
      (:A
        (Components|Activation|Activate (Variables|Default|GetFire) false)
        (Default|ConvertText (Variables|Default|GetAs%20UI%20Interaction)))
      (:B
        (Components|Activation|Deactivate (Variables|Default|GetFire))))
    (else
      (Default|ConvertText (Variables|Default|GetAs%20UI%20Interaction) (Variables|Default|GetText_Wood)))))

(fn ConstructionScript)