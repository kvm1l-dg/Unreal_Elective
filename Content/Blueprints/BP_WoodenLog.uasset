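; BP_WoodenLog is a wooden log pickup that a player can carry in the right hand.
; A collision sphere shows the pickup widget on overlap while the log is not held, and hides it on exit.
; Interact turns off physics, snaps the log to the player's hand socket and records it on the player, if none is attached.
; Both log-mesh overlap events set LogOverlap to false, and no drop logic exists here.
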(event OnComponentBeginOverlap(wooded_log_1)
  (params (OverlappedComponent :type Primitive%20Component%20Object%20Reference) (OtherActor :type Actor%20Object%20Reference) (OtherComp :type Primitive%20Component%20Object%20Reference) (OtherBodyIndex :type Integer) (bFromSweep :type Boolean) (SweepResult :type Hit%20Result%20Structure%20%28by%20ref%29))
  (Variables|Default|SetLog%20Overlap false))

(event OnComponentEndOverlap(Sphere_Collision)
  (params (OverlappedComponent :type Primitive%20Component%20Object%20Reference) (OtherActor :type Actor%20Object%20Reference) (OtherComp :type Primitive%20Component%20Object%20Reference) (OtherBodyIndex :type Integer))
  ;[0.15 0.003125 0.003125 0.5] Widget
  (Rendering|SetVisibility (Variables|Default|GetWidget_Pickup) false false))

(event OnComponentBeginOverlap(Sphere_Collision)
  (params (OverlappedComponent :type Primitive%20Component%20Object%20Reference) (OtherActor :type Actor%20Object%20Reference) (OtherComp :type Primitive%20Component%20Object%20Reference) (OtherBodyIndex :type Integer) (bFromSweep :type Boolean) (SweepResult :type Hit%20Result%20Structure%20%28by%20ref%29))
  ;[0.15 0.003125 0.003125 0.5] Widget
  (if (not (Variables|Default|GetLogInHand))
    (Rendering|SetVisibility (Variables|Default|GetWidget_Pickup) true false)))

(event OnComponentEndOverlap(wooded_log_1)
  (params (OverlappedComponent :type Primitive%20Component%20Object%20Reference) (OtherActor :type Actor%20Object%20Reference) (OtherComp :type Primitive%20Component%20Object%20Reference) (OtherBodyIndex :type Integer))
  (Variables|Default|SetLog%20Overlap false))

(event EventBeginPlay)

(event Collision|EventActorBeginOverlap
  (params (OtherActor :type Actor%20Object%20Reference)))

(event EventTick
  (params (DeltaSeconds :type Float%20%28single-precision%29)))

(event EventInteract
  (params (PlayerRef :type BP%20First%20Person%20Character%20Object%20Reference))
  ;[0 1 0.6087 0.5] Picking up the Log
  (if (not (Variables|/Game/FirstPerson/Blueprints/BP_FirstPersonCharacter.BP_FirstPersonCharacter_C|GetLog%20Attached%20 PlayerRef))
    (Physics|SetSimulatePhysics (Variables|Default|Getwooded_log_1) false)
    (Transformation|AttachComponentToComponent self (Variables|/Script/Engine.Character|GetMesh PlayerRef) "hand_rSocket" "SnapToTarget" "SnapToTarget" "SnapToTarget" true)
    (Variables|/Game/FirstPerson/Blueprints/BP_FirstPersonCharacter.BP_FirstPersonCharacter_C|SetLog%20Attached%20 PlayerRef true)
    (Variables|/Game/FirstPerson/Blueprints/BP_FirstPersonCharacter.BP_FirstPersonCharacter_C|SetWoodenLog PlayerRef self)
    (Variables|Default|SetLogInHand true)))

(fn ConstructionScript)